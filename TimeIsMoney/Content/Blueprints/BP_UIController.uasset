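; UI controller that shows the WBP_FinalUI widget and mouse cursor and runs a minutes-and-seconds countdown.
; BeginPlay seeds a short countdown, which Tick decrements about once per second through a latent Delay, setting OutOfTime when it runs out.
; Enter calls StartGame on the BP_Table_TimeIsMoney actor, independently of the timer.
; SpaceBar only prints a deprecation message.
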(event `self.ReceiveBeginPlay`
  (bind _returnvalue (`|CreateWidget` "/Game/UI/WBP_FinalUI.WBP_FinalUI_C"))
  (`UserWidget.AddToViewport` _returnvalue 0)
  (set `self.Seconds` 5)
  (set `self.Minutes` 0)
  (set `self.bShowMouseCursor` true))

(event `self.ReceiveTick`
  (params (DeltaSeconds :type "Float (single-precision)"))
  (`KismetSystemLibrary.Delay` 1.0)
  (set `self.Seconds` (- (`self.Seconds`) 1))
  (if (< (`self.Seconds`) 0)
    (set `self.Minutes` (- (`self.Minutes`) 1))
    (if (and (< (`self.Minutes`) 0) (< (`self.Seconds`) 0))
      (set `self.OutOfTime` true)
      (else
        (set `self.Seconds` 59)))))

(event `Key|SpaceBar`
  (params (Key :type "Key Structure"))
  (:`Pressed`
    (`KismetSystemLibrary.PrintString` "Depreciated")))

(event `Key|Enter`
  (params (Key :type "Key Structure"))
  (:`Pressed`
    (bind _returnvalue (`GameplayStatics.GetActorOfClass` "/Game/Blueprints/BP_Table_TimeIsMoney.BP_Table_TimeIsMoney_C"))
    (`CPP_Table_TimeIsMoney.StartGame` _returnvalue)))

(fn `UserConstructionScript`)