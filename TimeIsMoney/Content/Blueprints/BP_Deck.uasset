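; BP_Deck is a deck Blueprint that relays card draw and hand discard events to the WBP_FinalUI widget.
; On BeginPlay it binds handlers to its OnCardDrawn and OnHandDiscarded dispatchers.
; Each handler finds all top-level WBP_FinalUI widgets by class and calls DrawCard with the drawn card, or DiscardHand, printing a debug string.
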(event `OnHandDiscarded_Event`
  (bind _foundwidgets (`WidgetBlueprintLibrary.GetAllWidgetsOfClass` "/Game/UI/WBP_FinalUI.WBP_FinalUI_C"))
  (for _array_element _foundwidgets
    (`/Game/UI/WBP_FinalUI.DiscardHand` _array_element)
    (`KismetSystemLibrary.PrintString` "OnHandDiscarded Event")))

(event `self.ReceiveBeginPlay`
  (add `self.OnCardDrawn` (delegate `OnCardDrawn_Event`))
  (add `self.OnHandDiscarded` (delegate `OnHandDiscarded_Event`)))

(event `OnCardDrawn_Event` :!signature `self.OnCardDrawn`
  (params (DrawnCard :type "CPP_Card Object Reference"))
  (bind _foundwidgets (`WidgetBlueprintLibrary.GetAllWidgetsOfClass` "/Game/UI/WBP_FinalUI.WBP_FinalUI_C"))
  (for _array_element _foundwidgets
    (`/Game/UI/WBP_FinalUI.DrawCard` _array_element DrawnCard)
    (`KismetSystemLibrary.PrintString` "OnCardDrawn Event")))

(fn `UserConstructionScript`)