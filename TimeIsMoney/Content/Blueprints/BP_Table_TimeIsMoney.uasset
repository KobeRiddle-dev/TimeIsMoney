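; BP_Table_TimeIsMoney is the table for the Time Is Money card game, showing the cards played by the player and opponent.
; On BeginPlay it binds card-played and hand-start events and caches the opponent NPC.
; Each played card spawns as a BP_Card at that side's location and is tracked in PlayedCards.
; Hand start destroys them, using a while loop because removing during the ForEach skips elements.
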(event `OnHandStart_Event`
  (`self.DeletePlayedCards`))

(event `OnOppCardPlayed_Event` :!signature `self.OnOppCardPlayed`
  (params (CardPlayed :type "CPP_Card Object Reference"))
  (bind _newparam (`self.SpawnCard` CardPlayed (`self.Loc_OppCard`)))
  (`KismetArrayLibrary.Array_Add` (`self.PlayedCards`) _newparam))

(event `OnPlayerCardPlayed_Event` :!signature `self.OnPlayerCardPlayed`
  (params (CardPlayed :type "CPP_Card Object Reference"))
  (bind _newparam (`self.SpawnCard` CardPlayed (`self.Loc_PlayerCard`)))
  (`KismetArrayLibrary.Array_Add` (`self.PlayedCards`) _newparam))

(event `self.ReceiveBeginPlay`
  (add `self.OnPlayerCardPlayed` (delegate `OnPlayerCardPlayed_Event`))
  (add `self.OnOppCardPlayed` (delegate `OnOppCardPlayed_Event`))
  (add `self.OnHandStart` (delegate `OnHandStart_Event`))
  (bind _returnvalue (`GameplayStatics.GetActorOfClass` "/Game/Blueprints/BP_NPC_Opp_TimeIsMoney.BP_NPC_Opp_TimeIsMoney_C"))
  (set `self.Opponent` _returnvalue))

(fn `DeletePlayedCards`
  (bind _playedcards (`self.PlayedCards`))
  ;[1 1 1] this wouldn't delete all of the actors without this check for some reason
  (while (> (`KismetArrayLibrary.Array_Length` _playedcards) 0)
    (for (_array_element _array_index) _playedcards
      (`self.K2_DestroyActor` _array_element)
      (`KismetArrayLibrary.Array_Remove` _playedcards _array_index))))

(fn `SpawnCard`
  (params (CardSpawned :type "CPP_Card Object Reference") (SpawnLoc :type "Transform Structure"))
  (returns (NewParam :type "/Game/Blueprints/BP_Card Object Reference"))
  (bind _returnvalue (`|SpawnActorFromClass` "/Game/Blueprints/BP_Card.BP_Card_C" SpawnLoc "Undefined" "MultiplyWithRoot" null null))
  (`CPP_Card.InitializeCard` _returnvalue (`CPP_Card.CardSuit` CardSpawned) (`CPP_Card.CardNumber` CardSpawned))
  (return _returnvalue))

(fn `UserConstructionScript`)