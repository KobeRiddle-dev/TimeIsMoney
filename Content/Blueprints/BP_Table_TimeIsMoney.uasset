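; BP_Table_TimeIsMoney is the card table that visualizes a player-versus-opponent card game and relays results to the UI.
; BeginPlay binds game events for cards played, hand start, winner determined and game end.
; Played cards spawn as BP_Card actors, pause, then slide to discard spots via timeline lerps, and are destroyed at next hand start.
; Winner and game-end events update WBP_FinalUI, with game end also clearing the card array.
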(event `OnGameEnded_Event` :!signature `self.OnGameEnded`
  (params (PlayerIsWin :type Boolean))
  (bind _foundwidgets (`WidgetBlueprintLibrary.GetAllWidgetsOfClass` "/Game/UI/WBP_FinalUI.WBP_FinalUI_C"))
  (for _array_element _foundwidgets
    (`/Game/UI/WBP_FinalUI.EndGame` _array_element PlayerIsWin)
    (`KismetArrayLibrary.Array_Clear` (`self.SpawnedCards`))))

(event `OnWinnerDetermined_Event`
  (bind _foundwidgets (`WidgetBlueprintLibrary.GetAllWidgetsOfClass` "/Game/UI/WBP_FinalUI.WBP_FinalUI_C"))
  (for _array_element _foundwidgets
    (`/Game/UI/WBP_WinResults.UpdateWins` (`/Game/UI/WBP_FinalUI.WBP_WinResults` _array_element) self)))

(event `OnHandStart_Event`
  (`self.DeleteSpawnedCards`))

(event `OnPlayerCardPlayed_Event` :!signature `self.OnPlayerCardPlayed`
  (params (CardPlayed :type "CPP_Card Object Reference"))
  (bind _loc_playercard (`self.Loc_PlayerCard`))
  (bind _cardspawned (`self.SpawnCard` CardPlayed _loc_playercard))
  (`KismetSystemLibrary.Delay` 1.0)
  (bind (_direction _movement) (`Timeline|Timeline` :!via `PlayFromStart`)
    (:`Update`
      (`self.K2_SetActorLocation` _cardspawned (`KismetMathLibrary.VLerp` (.location _loc_playercard) (.location (`self.Loc_PlayerDiscard`)) _movement) false false))))

(event `OnOppCardPlayed_Event` :!signature `self.OnOppCardPlayed`
  (params (CardPlayed :type "CPP_Card Object Reference"))
  (bind _loc_oppcard (`self.Loc_OppCard`))
  (bind _cardspawned (`self.SpawnCard` CardPlayed _loc_oppcard))
  (`KismetSystemLibrary.Delay` 1.0)
  (bind (_direction _movement) (`Timeline|Timeline_0` :!via `PlayFromStart`)
    (:`Update`
      (`self.K2_SetActorLocation` _cardspawned (`KismetMathLibrary.VLerp` (.location _loc_oppcard) (.location (`self.Loc_OppDiscard`)) _movement) false false))))

(event `self.ReceiveBeginPlay`
  (add `self.OnOppCardPlayed` (delegate `OnOppCardPlayed_Event`))
  (add `self.OnPlayerCardPlayed` (delegate `OnPlayerCardPlayed_Event`))
  (add `self.OnHandStart` (delegate `OnHandStart_Event`))
  (add `self.OnWinnerDetermined` (delegate `OnWinnerDetermined_Event`))
  (add `self.OnGameEnded` (delegate `OnGameEnded_Event`)))

(fn `DeleteSpawnedCards`
  (bind _spawnedcards (`self.SpawnedCards`))
  (bind _returnvalue (`KismetArrayLibrary.Array_Length` _spawnedcards))
  (`KismetSystemLibrary.PrintString` (`KismetStringLibrary.Conv_IntToString` _returnvalue))
  (while (> _returnvalue 0)
    (for (_array_element _array_index) _spawnedcards
      (`self.K2_DestroyActor` _array_element)
      (`KismetArrayLibrary.Array_Remove` _spawnedcards _array_index))))

(fn `DiscardHand`)

(fn `SpawnCard`
  (params (Card :type "CPP_Card Object Reference") (SpawnLoc :type "Transform Structure"))
  (returns (CardSpawned :type "CPP_Card Object Reference"))
  (bind _returnvalue (`|SpawnActorFromClass` "/Game/Blueprints/BP_Card.BP_Card_C" SpawnLoc "Undefined" "MultiplyWithRoot" null null))
  (`CPP_Card.InitializeCard` _returnvalue (`CPP_Card.CardSuit` Card) (`CPP_Card.CardNumber` Card))
  (`KismetArrayLibrary.Array_Add` (`self.SpawnedCards`) _returnvalue)
  (return _returnvalue))

(fn `UserConstructionScript`)