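; Player controller that sets up the game UI and runs a minutes-and-seconds countdown.
; On possessing BP_firstpersonCharacter, it shows the mouse cursor, adds WBP_FinalUI to the viewport and calls its StartGame; the countdown values reset on any possession.
; Tick uses a one-second Delay as a makeshift timer, rolling seconds into minutes and setting OutOfTime when both run out.
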(event `self.ReceivePossess`
  (params (PossessedPawn :type "Pawn Object Reference"))
  (set `self.Seconds` 5)
  (set `self.Minutes` 0)
  (cast `/Game/Blueprints/Firstperson_blueprints/FirstPerson/Blueprints/BP_firstpersonCharacter` PossessedPawn)
  (set `self.bShowMouseCursor` true)
  (bind _returnvalue (`|CreateWidget` "/Game/UI/WBP_FinalUI.WBP_FinalUI_C" (`GameplayStatics.GetPlayerController` 0)))
  (`UserWidget.AddToViewport` _returnvalue 0)
  (`/Game/UI/WBP_FinalUI.StartGame` _returnvalue)
  (set `self.bShowMouseCursor` true))

(event `self.ReceiveTick`
  (params (DeltaSeconds :type "Float (single-precision)"))
  (`KismetSystemLibrary.Delay` 1.0)
  (set `self.Seconds` (- (`self.Seconds`) 1))
  (if (< (`self.Seconds`) 0)
    (set `self.Minutes` (- (`self.Minutes`) 1))
    (if (and (< (`self.Minutes`) 0) (< (`self.Seconds`) 0))
      (set `self.OutOfTime` true)
      (else
        (set `self.Seconds` 59)))))

(fn `UserConstructionScript`)